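; BP_weapon is a hitscan weapon that handles firing and reloading for its owning Pawn, using a weapon stats struct.
; StartShooting checks death, reload state and ammo, spends a round, flags the pawn as shooting, and line-traces from the camera along base aim.
; Hit BP_BasePawn actors receive the weapon's damage, and each trace draws a debug line.
; StartReload clears the reloading flag and instantly refills the magazine if the pawn is alive.
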(fn `StartReload`
  (bind _pawn (`self.Pawn`))
  (bind _structure_stats_weapon (`self.Structure_Stats_Weapon`))
  (set `/Game/Blueprint/Character/BP_BasePawn.Reloading` false _pawn)
  (if (not (`/Game/Blueprint/Character/BP_BasePawn.Death?` _pawn))
    (bind _structout (setmembers `/Game/Blueprint/Weapon/Structure_Stats_weapon` :`StructRef` _structure_stats_weapon :`MagazineCurrent` (`.MagazineCapacity_9_74FCFD004BEB2EC3E74BD7BFBAAD8D9C` (break `/Game/Blueprint/Weapon/Structure_Stats_weapon` _structure_stats_weapon))))
    (set `self.Structure_Stats_Weapon` _structout)))

(fn `StartShooting`
  (bind _pawn (`self.Pawn`))
  (bind _pawn_2 (`self.Pawn`))
  (bind _pawn_3 (`self.Pawn`))
  (bind ((`MagazineCurrent_10_50C8E4BC4DB14EAB99592D8B8490750C` _magazinecurrent)) (break `/Game/Blueprint/Weapon/Structure_Stats_weapon` (`self.Structure_Stats_Weapon`)))
  (bind _returnvalue (`SceneComponent.K2_GetComponentLocation` (`/Game/Blueprint/Character/BP_BasePawn.FPSCamera` _pawn_2)))
  (if (and (not (`/Game/Blueprint/Character/BP_BasePawn.Death?` _pawn)) (> _magazinecurrent 0) (not (`/Game/Blueprint/Character/BP_BasePawn.Reloading` _pawn)))
    (bind _result (`/Engine/EditorBlueprintResources/StandardMacros.DecrementInt` _magazinecurrent)
      (:`  `
        (bind _structout (setmembers `/Game/Blueprint/Weapon/Structure_Stats_weapon` :`StructRef` (`self.Structure_Stats_Weapon`) :`MagazineCurrent` _result))
        (set `self.Structure_Stats_Weapon` _structout)
        (set `/Game/Blueprint/Character/BP_BasePawn.Shooting` true (`self.Pawn`))
        (bind _outhit (`KismetSystemLibrary.LineTraceSingleForObjects` _returnvalue (+ _returnvalue (* (`KismetMathLibrary.GetForwardVector` (`Pawn.GetBaseAimRotation` _pawn_2)) (`.BulletDistance_13_C491C2BC454A326AF1E4658917A83251` (break `/Game/Blueprint/Weapon/Structure_Stats_weapon` (`self.Structure_Stats_Weapon`))))) (`|MakeArray` "ObjectTypeQuery1" "ObjectTypeQuery2" "ObjectTypeQuery3" :!type "EObjectTypeQuery Enum") false (`|MakeArray` (`/Game/Blueprint/Character/BP_BasePawn.Weapon` _pawn_3) _pawn_3 :!type "Actor Object Reference") "ForDuration" true (struct :`R` 0.148977 :`B` 1.0 :`A` 1.0) (struct :`G` 1.0 :`A` 1.0) 2.0))
        (bind _asbp_base_pawn (cast `/Game/Blueprint/Character/BP_BasePawn` (`.HitActor` (`GameplayStatics.BreakHitResult` _outhit))))
        (`/Game/Blueprint/Character/BP_BasePawn.AnyDamage` _asbp_base_pawn (`.Damage_2_6E6B255F41D971672F8304965FFA14AE` (break `/Game/Blueprint/Weapon/Structure_Stats_weapon` (`self.Structure_Stats_Weapon`))))))))

(fn `UserConstructionScript`)