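; AI controller for enemy pawns that runs the BT_Enemy behavior tree on possession and feeds its blackboard.
; AI perception flags any sensed pawn from another team as the seen enemy and stores it for the tree.
; It starts in aggressive mode and switches to retreat when SetMode receives low health.
; Events to set and clear focus wrap the controller's focus calls.
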(event `FocusTarget`
  (params (NewFocus :type "Actor Object Reference"))
  ;[1 1 1] focusing
  (`self.K2_SetFocus` NewFocus))

(event `self.ReceivePossess`
  (params (PossessedPawn :type "Pawn Object Reference"))
  ;[1 1 1] init. posses
  (`self.iniPosses` PossessedPawn))

(event `ClearTarget`
  ;[1 1 1] focusing
  (`self.K2_ClearFocus`))

(event `self.AIPerception.OnTargetPerceptionUpdated`
  (params (Actor :type "Actor Object Reference") (Stimulus :type "AIStimulus Structure"))
  (bind _returnvalue (`AIBlueprintHelperLibrary.GetBlackboard` self))
  (bind _asbp_base_pawn (cast `/Game/Blueprint/Character/BP_BasePawn` Actor))
  (if (not (== (`/Game/Blueprint/Character/BP_BasePawn.TeamID` _asbp_base_pawn) (`/Game/Blueprint/Character/BP_BasePawn.TeamID` (`self.AI_Pawn`))))
    (`BlackboardComponent.SetValueAsBool` _returnvalue "EnemySeen?" true)
    (`BlackboardComponent.SetValueAsObject` _returnvalue "EnemyPawn" _asbp_base_pawn)))

(event `SetMode`
  (params (Heatlh :type "Float (double-precision)"))
  (if (<= Heatlh 30.0)
    (`BlackboardComponent.SetValueAsBool` (`AIBlueprintHelperLibrary.GetBlackboard` self) "AggressiveMode" false)
    (`BlackboardComponent.SetValueAsBool` (`AIBlueprintHelperLibrary.GetBlackboard` self) "RetreatMode" true)))

(event `self.ReceiveBeginPlay`
  (`BlackboardComponent.SetValueAsBool` (`AIBlueprintHelperLibrary.GetBlackboard` self) "AggressiveMode" true))

(fn `iniPosses`
  (params (pawn :type "Pawn Object Reference"))
  (bind _asbp_base_pawn (cast `/Game/Blueprint/Character/BP_BasePawn` pawn))
  (set `self.AI_Pawn` _asbp_base_pawn)
  (`self.RunBehaviorTree` "/Game/Blueprint/AI/Main/BT_Enemy.BT_Enemy"))

(fn `UserConstructionScript`)