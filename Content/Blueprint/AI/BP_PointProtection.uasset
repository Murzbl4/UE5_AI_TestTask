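; BP_PointProtection is a trigger zone that switches enemy AI into point defense when a pawn enters its Box.
; On overlap by a BP_BasePawn, it scans all such pawns for AI-controlled ones with a different TeamID from the intruder.
; Their blackboards get PointProtection set and AggressiveMode cleared, with no reset in this Blueprint.
; It also prints every overlapping actor's name.
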(event `self.Box.OnComponentBeginOverlap`
  (params (OverlappedComponent :type "PrimitiveComponent Object Reference") (OtherActor :type "Actor Object Reference") (OtherComp :type "PrimitiveComponent Object Reference") (OtherBodyIndex :type Integer) (bFromSweep :type Boolean) (SweepResult :type "HitResult Structure (by ref)"))
  (`KismetSystemLibrary.PrintString` (`KismetSystemLibrary.GetDisplayName` OtherActor))
  (bind _asbp_base_pawn (cast `/Game/Blueprint/Character/BP_BasePawn` OtherActor))
  (bind _outactors (`GameplayStatics.GetAllActorsOfClass` "/Game/Blueprint/Character/BP_BasePawn.BP_BasePawn_C"))
  (for _array_element _outactors
    (`/Engine/EditorBlueprintResources/StandardMacros.IsValid` (`AIBlueprintHelperLibrary.GetAIController` _array_element)
      (:`Is Valid`
        (if (not (== (`/Game/Blueprint/Character/BP_BasePawn.TeamID` _asbp_base_pawn) (`/Game/Blueprint/Character/BP_BasePawn.TeamID` _array_element)))
          (bind _returnvalue (`AIBlueprintHelperLibrary.GetBlackboard` (`AIBlueprintHelperLibrary.GetAIController` _array_element)))
          (`BlackboardComponent.SetValueAsBool` _returnvalue "PointProtection" true)
          (`BlackboardComponent.SetValueAsBool` _returnvalue "AggressiveMode" false))))))

(fn `UserConstructionScript`)