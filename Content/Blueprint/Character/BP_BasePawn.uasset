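; BP_BasePawn is a shooter character for player and AI, with separate first-person arms and third-person body.
; On BeginPlay it spawns a weapon attached to both meshes, adds screen UI and optionally randomizes its team.
; Input drives firing and delayed reloading, while Cover and Attack events toggle crouch.
; Damage updates the health bar; only non-player pawns switch AI mode, ragdoll at zero health and are destroyed with their weapon.
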(event `InputAction|Reload`
  (params (Key :type "Key Structure"))
  (:`Pressed`
    (`KismetSystemLibrary.K2_SetTimer` (`self.Weapon`) "StartReload" 2.0)))

(event `InputAction|Fire`
  (params (Key :type "Key Structure"))
  (:`Pressed`
    (`/Game/Blueprint/Weapon/BP_weapon.StartShooting` (`self.Weapon`))))

(event `AnyDamage`
  (params (Damage :type "Float (double-precision)"))
  (bind _output_get (set `self.HPCurrent` (- (`self.HPCurrent`) Damage)))
  (`self.Change_HealthBar`)
  (cast `/Game/Blueprint/Character/BP_Controller` (`self.GetController`)
    (:`CastFailed`
      (bind _asbp_ai_controller (cast `/Game/Blueprint/AI/Main/BP_Ai_Controller` (`AIBlueprintHelperLibrary.GetAIController` self)))
      (`/Game/Blueprint/AI/Main/BP_Ai_Controller.SetMode` _asbp_ai_controller 0.0)
      (if (<= _output_get 0.0)
        (set `self.Death?` true)
        (`self.MakeRagdoll`)
        (`KismetSystemLibrary.Delay` 5.0)
        (`self.K2_DestroyActor` self)
        (`self.K2_DestroyActor` (`self.Weapon`))))))

(event `self.ReceiveBeginPlay`
  (bind _returnvalue (`|SpawnActorFromClass` "/Game/Blueprint/Weapon/BP_weapon.BP_weapon_C" (`KismetMathLibrary.MakeTransform` (0.0 0.0 0.0)) "Undefined" "MultiplyWithRoot" null null))
  (set `/Game/Blueprint/Weapon/BP_weapon.Pawn` self _returnvalue)
  (set `self.Weapon` _returnvalue)
  (`self.Change_HealthBar`)
  (`self.AttachGunToPerson`)
  (`self.AddUIOnScreen`)
  (`self.JoinRandomTeam`))

(event `AttachGunToPerson`
  (bind _weapon (`self.Weapon`))
  (`SceneComponent.K2_AttachToComponent` (`/Game/Blueprint/Weapon/BP_weapon.SM_Weapon_FPS` _weapon) (`self.Arms`) "Socket_AK74" "SnapToTarget" "SnapToTarget" "KeepRelative" true)
  (`SceneComponent.K2_AttachToComponent` (`/Game/Blueprint/Weapon/BP_weapon.SM_Weapon_TPS` _weapon) (`self.Mesh`) "Socket_AK74" "SnapToTarget" "SnapToTarget" "KeepRelative" true))

(event `/Game/Blueprint/AI/Interface/I_Combat.Cover`
  (`self.Crouch`))

(event `/Game/Blueprint/AI/Interface/I_Combat.Attack`
  (`self.UnCrouch`))

(fn `AddUIOnScreen`
  (bind _returnvalue (`|CreateWidget` "/Game/Blueprint/Widget/W_UI.W_UI_C"))
  (`UserWidget.AddToViewport` _returnvalue 0))

(fn `Change_HealthBar`
  (bind _w_healthbar (`self.W_HealthBar`))
  (bind _asw_health_bar (cast `/Game/Blueprint/Widget/W_HealthBar` (`WidgetComponent.GetWidget` _w_healthbar)))
  (`ProgressBar.SetPercent` (`/Game/Blueprint/Widget/W_HealthBar.ProgressBar_103` _asw_health_bar) (/ (`self.HPCurrent`) (`self.HPMax`)))
  (if (<= (`self.HPCurrent`) 0.0)
    (`SceneComponent.SetHiddenInGame` _w_healthbar true false)))

(fn `JoinRandomTeam`
  (if (`self.RandomTeam?`)
    (set `self.TeamID` (`KismetMathLibrary.RandomIntegerInRange` 0 3)))
  (`TextRenderComponent.K2_SetText` (`self.TextRender`) (`KismetTextLibrary.Conv_IntToText` (`self.TeamID`))))

(fn `MakeRagdoll`
  (bind _mesh (`self.Mesh`))
  (`MovementComponent.StopMovementImmediately` (`self.CharacterMovement`))
  (`PrimitiveComponent.SetSimulatePhysics` _mesh true)
  (`SkeletalMeshComponent.SetAllBodiesBelowSimulatePhysics` _mesh "pelvis" true true))

(fn `UserConstructionScript`
  (`PrimitiveComponent.SetOwnerNoSee` (`self.Mesh`) true)
  (`PrimitiveComponent.SetOnlyOwnerSee` (`self.Arms`) true)
  (`TextRenderComponent.K2_SetText` (`self.TextRender`) (`KismetTextLibrary.Conv_IntToText` (`self.TeamID`))))